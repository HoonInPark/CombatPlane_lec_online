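; Showcase Blueprint for the West MQ-1 UAV that exposes its moving parts and appearance to generic slider and checkbox controls.
; Single sliders drive propeller speed and blades, rudder and light emissivity, while a checkbox toggles the damaged look.
; Twin sliders handle landing gear, sensor rotation and pitch, flaps and stabilizers, with rear wheels sharing one value and left stabilizer input negated.
; It only forwards values to setter functions defined outside this graph.
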(event EventBeginPlay
  (|CallParentFunction) ; This node is disabled and will not be called.\nDrag off pins to build functionality.
)

(event Collision|EventActorBeginOverlap
  (params (OtherActor :type Actor%20Object%20Reference))
  (|CallParentFunction OtherActor) ; This node is disabled and will not be called.\nDrag off pins to build functionality.
)

(event EventSetTwinSliderVariable3
  (params (bFirstSlider? :type Boolean) (NewFirstValue :type Float%20%28double-precision%29) (NewSecondValue :type Float%20%28double-precision%29))
  (CallFunction|SetStabilizersL (* NewFirstValue -1.0))
  (CallFunction|SetStabilizersR NewSecondValue))

(event EventSetTwinSliderVariable1
  (params (bFirstSlider? :type Boolean) (NewFirstValue :type Float%20%28double-precision%29) (NewSecondValue :type Float%20%28double-precision%29))
  (CallFunction|SetSensorRotation NewFirstValue)
  (CallFunction|SetSensorPitch NewSecondValue))

(event EventSetCheckboxVariable0
  (params (NewState :type Boolean))
  (CallFunction|SetShowDamaged NewState))

(event EventTick
  (params (DeltaSeconds :type Float%20%28single-precision%29))
  (|CallParentFunction DeltaSeconds) ; This node is disabled and will not be called.\nDrag off pins to build functionality.
)

(event EventSetSliderVariable0
  (params (NewValue :type Float%20%28double-precision%29))
  (CallFunction|SetPropellerSpeed NewValue))

(event EventSetSliderVariable1
  (params (NewValue :type Float%20%28double-precision%29))
  (CallFunction|SetPropellerBlades NewValue))

(event EventSetSliderVariable2
  (params (NewValue :type Float%20%28double-precision%29))
  (CallFunction|SetRudder NewValue))

(event EventSetSliderVariable3
  (params (NewValue :type Float%20%28double-precision%29))
  (CallFunction|SetLightsEmissivity NewValue))

(event EventSetTwinSliderVariable2
  (params (bFirstSlider? :type Boolean) (NewFirstValue :type Float%20%28double-precision%29) (NewSecondValue :type Float%20%28double-precision%29))
  (CallFunction|SetFlapsL NewFirstValue)
  (CallFunction|SetFlapsR NewSecondValue))

(event EventSetTwinSliderVariable0
  (params (bFirstSlider? :type Boolean) (NewFirstValue :type Float%20%28double-precision%29) (NewSecondValue :type Float%20%28double-precision%29))
  (CallFunction|RetractFrontWheel NewFirstValue)
  (CallFunction|RetractRearLWheel NewSecondValue)
  (CallFunction|RetractRearRWheel NewSecondValue))

(fn ConstructionScript
  (|CallParentFunction))